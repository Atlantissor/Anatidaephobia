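; Collectible duck actor that varies its look between clean, dirty and burned texture sets; it contains no pickup logic.
; The Construction Script creates a dynamic material instance on the Duck mesh and applies a random set of color, roughness/metallic and normal textures.
; BeginPlay picks again, always using the burned set when the Oven flag is true, so the look seen in editor can differ at runtime.
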(event Collision|EventActorBeginOverlap
  (params (OtherActor :type Actor%20Object%20Reference)))

(event EventBeginPlay
  (if (Variables|Default|Getoven)
    (Variables|Default|SetRandTextureColor "/Game/Textures/T_Collectible_Burned_BaseColor.T_Collectible_Burned_BaseColor" :!label _label)
    (Variables|Default|SetRandTextureRough "/Game/Textures/T_Collectible_Burned_OcclusionRoughnessMetallic.T_Collectible_Burned_OcclusionRoughnessMetallic")
    (Variables|Default|SetRandTextureNorm "/Game/Textures/T_Collectible_Burned_Normal.T_Collectible_Burned_Normal")
    (else
      (bind _output_get (Variables|Default|SetRandomNumber (Math|Random|RandomIntegerinRange 0 2)))
      (if (== _output_get 0)
        (Variables|Default|SetRandTextureColor "/Game/Textures/T_Collectible_BaseColor.T_Collectible_BaseColor")
        (Variables|Default|SetRandTextureRough "/Game/Textures/T_Collectible_OcclusionRoughnessMetallic.T_Collectible_OcclusionRoughnessMetallic")
        (Variables|Default|SetRandTextureNorm 0)
        (elif (== _output_get 1)
          (Variables|Default|SetRandTextureColor "/Game/Textures/T_Collectible_Dirty_BaseColor.T_Collectible_Dirty_BaseColor")
          (Variables|Default|SetRandTextureRough "/Game/Textures/T_Collectible_Dirty_OcclusionRoughnessMetallic.T_Collectible_Dirty_OcclusionRoughnessMetallic")
          (Variables|Default|SetRandTextureNorm "/Game/Textures/T_Collectible_Dirty_Normal.T_Collectible_Dirty_Normal")
          (else
            (goto _label))))))
  (Rendering|Material|SetTextureParameterValue (Variables|Default|GetDuckMatInst) "color" (Variables|Default|GetRandTextureColor))
  (Rendering|Material|SetTextureParameterValue (Variables|Default|GetDuckMatInst) "metRoug" (Variables|Default|GetRandTextureRough))
  (Rendering|Material|SetTextureParameterValue (Variables|Default|GetDuckMatInst) "normal" (Variables|Default|GetRandTextureNorm)))

(fn ConstructionScript
  (bind _returnvalue (Rendering|Material|CreateDynamicMaterialInstance (Variables|Default|Getduck) 0 "/Game/Materials/M_Collectible_Inst.M_Collectible_Inst" "None" :!class /Script/Engine.PrimitiveComponent))
  (bind _output_get (Variables|Default|SetDuckMatInst _returnvalue))
  (Rendering|Material|SetMaterial (Variables|Default|Getduck) 0 _output_get)
  (bind _output_get_2 (Variables|Default|SetRandomNumber (Math|Random|RandomIntegerinRange 0 2)))
  (if (== _output_get_2 0)
    (Variables|Default|SetRandTextureColor "/Game/Textures/T_Collectible_BaseColor.T_Collectible_BaseColor")
    (Variables|Default|SetRandTextureRough "/Game/Textures/T_Collectible_OcclusionRoughnessMetallic.T_Collectible_OcclusionRoughnessMetallic")
    (Variables|Default|SetRandTextureNorm 0)
    (elif (== _output_get_2 1)
      (Variables|Default|SetRandTextureColor "/Game/Textures/T_Collectible_Dirty_BaseColor.T_Collectible_Dirty_BaseColor")
      (Variables|Default|SetRandTextureRough "/Game/Textures/T_Collectible_Dirty_OcclusionRoughnessMetallic.T_Collectible_Dirty_OcclusionRoughnessMetallic")
      (Variables|Default|SetRandTextureNorm "/Game/Textures/T_Collectible_Dirty_Normal.T_Collectible_Dirty_Normal")
      (else
        (Variables|Default|SetRandTextureColor "/Game/Textures/T_Collectible_Burned_BaseColor.T_Collectible_Burned_BaseColor")
        (Variables|Default|SetRandTextureRough "/Game/Textures/T_Collectible_Burned_OcclusionRoughnessMetallic.T_Collectible_Burned_OcclusionRoughnessMetallic")
        (Variables|Default|SetRandTextureNorm "/Game/Textures/T_Collectible_Burned_Normal.T_Collectible_Burned_Normal"))))
  (Rendering|Material|SetTextureParameterValue (Variables|Default|GetDuckMatInst) "color" (Variables|Default|GetRandTextureColor))
  (Rendering|Material|SetTextureParameterValue (Variables|Default|GetDuckMatInst) "metRoug" (Variables|Default|GetRandTextureRough))
  (Rendering|Material|SetTextureParameterValue (Variables|Default|GetDuckMatInst) "normal" (Variables|Default|GetRandTextureNorm)))