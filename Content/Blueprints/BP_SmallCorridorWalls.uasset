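; Small corridor wall set of nine static meshes that randomizes its wall color and window placement.
; The construction script applies one shared dynamic M_Wall1 instance with a random color to the "Wall" slot.
; BeginPlay rerolls the color onto per-mesh dynamic instances and sets fixed materials on the other slots.
; Both passes independently give two segments a roughly one-in-five window chance, so runtime can differ from the construction result.
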(event EventBeginPlay
  (bind _minvalue (Variables|Default|GetMinValue))
  (Variables|Default|SetWallColor (Utilities|Struct|MakeLinearColor (Math|Random|RandomFloatinRange _minvalue 0.9) (Math|Random|RandomFloatinRange _minvalue 0.9) (Math|Random|RandomFloatinRange _minvalue 0.9) 1.0))
  (for _array_element (Utilities|Array|MakeArray (Variables|Default|GetStaticMesh) (Variables|Default|GetStaticMesh2) (Variables|Default|GetStaticMesh3) (Variables|Default|GetStaticMesh4) (Variables|Default|GetStaticMesh5) (Variables|Default|GetStaticMesh6) (Variables|Default|GetStaticMesh7) (Variables|Default|GetStaticMesh1) (Variables|Default|GetStaticMesh8))
    (bind _output_get (Variables|Default|SetCurrentArrayElement _array_element))
    (bind _returnvalue (Rendering|Material|CreateDynamicMaterialInstance _output_get 1 0 "None" :!class /Script/Engine.PrimitiveComponent))
    (bind _output_get_2 (Variables|Default|SetMatInst _returnvalue))
    (Rendering|Material|SetVectorParameterValue _output_get_2 "Color" (Variables|Default|GetWallColor) :!class /Script/Engine.MaterialInstanceDynamic)
    (Rendering|Material|SetMaterial (Variables|Default|GetCurrentArrayElement) 0 "/Game/Materials/M_Wall2.M_Wall2")
    (Rendering|Material|SetMaterial (Variables|Default|GetCurrentArrayElement) 2 "/Game/Materials/M_WallPlastic.M_WallPlastic"))
  (for _array_element_2 (Utilities|Array|MakeArray (Variables|Default|GetStaticMesh3) (Variables|Default|GetStaticMesh8))
    (if (> (Math|Random|RandomIntegerinRange 0 100) 80)
      (Components|StaticMesh|SetStaticMesh _array_element_2 "/Game/assets_replaced/SM_Mur_Fenetre.SM_Mur_Fenetre")
      (else
        (Components|StaticMesh|SetStaticMesh _array_element_2 "/Game/assets_replaced/SM_Mur_Petit.SM_Mur_Petit")))))

(fn ConstructionScript
  (bind _minvalue (Variables|Default|GetMinValue))
  (Variables|Default|SetWallColor (Utilities|Struct|MakeLinearColor (Math|Random|RandomFloatinRange _minvalue 1.0) (Math|Random|RandomFloatinRange _minvalue 1.0) (Math|Random|RandomFloatinRange _minvalue 1.0) 1.0))
  (bind _returnvalue (Rendering|Material|CreateDynamicMaterialInstance "/Game/Materials/M_Wall1.M_Wall1" "None" :!class /Script/Engine.KismetMaterialLibrary))
  (Variables|Default|SetMatInst _returnvalue)
  (for _array_element (Utilities|Array|MakeArray (Variables|Default|GetStaticMesh) (Variables|Default|GetStaticMesh2) (Variables|Default|GetStaticMesh3) (Variables|Default|GetStaticMesh4) (Variables|Default|GetStaticMesh5) (Variables|Default|GetStaticMesh6) (Variables|Default|GetStaticMesh7) (Variables|Default|GetStaticMesh1) (Variables|Default|GetStaticMesh8))
    (Rendering|Material|SetMaterialbyName _array_element "Wall" (Variables|Default|GetMatInst))
    (Rendering|Material|SetVectorParameterValue (Variables|Default|GetMatInst) "Color" (Variables|Default|GetWallColor) :!class /Script/Engine.MaterialInstanceDynamic))
  (for _array_element_2 (Utilities|Array|MakeArray (Variables|Default|GetStaticMesh3) (Variables|Default|GetStaticMesh8))
    (if (> (Math|Random|RandomIntegerinRange 0 100) 80)
      (Components|StaticMesh|SetStaticMesh _array_element_2 "/Game/assets_replaced/SM_Mur_Fenetre.SM_Mur_Fenetre")
      (else
        (Components|StaticMesh|SetStaticMesh _array_element_2 "/Game/assets_replaced/SM_Mur_Petit.SM_Mur_Petit")))))