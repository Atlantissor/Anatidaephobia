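; BP_Stalker is an enemy actor that raises the player character's Fear whenever it has line of sight to them.
; A delay loop repeatedly traces on the Camera channel toward a jittered player position, adding Fear on hits until it passes the limit, then calls Watched and stops.
; A looping timer, its period randomized once at BeginPlay, runs IsAlive to teleport the stalker to a random preset location and yaw.
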(event EventBeginPlay
  (Utilities|Time|SetTimerbyFunctionName 0 "IsAlive" (Math|Random|RandomFloatinRange 5.0 3e+01) true)
  (bind _outhit (Collision|LineTraceByChannel (Transformation|GetWorldLocation (Variables|Default|GetDefaultSceneRoot)) (+ (Transformation|GetWorldLocation (Variables|/Script/Engine.Actor|GetRootComponent (Game|GetPlayerCharacter 0))) (Math|Vector|MakeVector (Math|Random|RandomFloatinRange -1e+01 1e+01) (Math|Random|RandomFloatinRange -1e+01 1e+01) (Math|Random|RandomFloatinRange -1e+01 1e+01))) "TraceTypeQuery2" false 0 "None" :!label _label))
  (bind _asthird_person_character (Utilities|Casting|CastToThirdPersonCharacter (.HitActor (Collision|BreakHitResult _outhit)))
    (:then
      (if (<= (Variables|/Game/ThirdPersonBP/Blueprints/ThirdPersonCharacter.ThirdPersonCharacter_C|GetFear _asthird_person_character) 1e+02)
        (Variables|/Game/ThirdPersonBP/Blueprints/ThirdPersonCharacter.ThirdPersonCharacter_C|SetFear _asthird_person_character (+ (Variables|/Game/ThirdPersonBP/Blueprints/ThirdPersonCharacter.ThirdPersonCharacter_C|GetFear _asthird_person_character) 1.5))
        (Utilities|FlowControl|Delay 0.1 :!label _label_2)
        (goto _label)
        (else
          (Default|Watched _asthird_person_character))))
    (:CastFailed
      (goto _label_2))))

(event EventTick
  (params (DeltaSeconds :type Float%20%28single-precision%29)))

(fn ConstructionScript)

(fn IsAlive
  (bind _newvar_0 (Variables|Default|GetNewVar_0))
  (bind _newvar_1 (Variables|Default|GetNewVar_1))
  (bind _newvar_10 (Variables|Default|GetNewVar_10))
  (bind _newvar_2 (Variables|Default|GetNewVar_2))
  (bind _newvar_3 (Variables|Default|GetNewVar_3))
  (bind _newvar_4 (Variables|Default|GetNewVar_4))
  (bind _newvar_5 (Variables|Default|GetNewVar_5))
  (bind _newvar_6 (Variables|Default|GetNewVar_6))
  (bind _newvar_7 (Variables|Default|GetNewVar_7))
  (bind _newvar_8 (Variables|Default|GetNewVar_8))
  (bind _newvar_9 (Variables|Default|GetNewVar_9))
  (bind _array (Utilities|Array|MakeArray _newvar_0 _newvar_1 _newvar_2 _newvar_3 _newvar_4 _newvar_5 _newvar_6 _newvar_7 _newvar_8 _newvar_9 _newvar_10))
  (Transformation|SetActorLocation (Utilities|Array|Get(acopy) _array (Math|Random|RandomInteger (Utilities|Array|Length _array))) false false)
  (Transformation|SetActorRotation (Math|Rotator|MakeRotator 0.0 0.0 (Math|Random|RandomFloatinRange 0.0 3.6e+02))))